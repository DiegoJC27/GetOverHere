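; BP_Bullet is a projectile actor that travels at a set speed for a limited lifetime.
; Each Tick counts down TimeLeft and advances the root component's relative X by Speed times delta time, without sweep or collision logic.
; When time runs out it calls ActivateEvent(false) on BPSetActiveComponent instead of destroying itself.
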(event `self.ReceiveTick`
  (params (DeltaSeconds :type "Float (single-precision)"))
  (bind _defaultsceneroot (`self.DefaultSceneRoot`))
  (bind (_relativelocation_x _relativelocation_y _relativelocation_z) (`KismetMathLibrary.BreakVector` (`SceneComponent.RelativeLocation` _defaultsceneroot)))
  (bind _output_get (set `self.TimeLeft` (- (`self.TimeLeft`) DeltaSeconds)))
  (if (> _output_get 0.0)
    (`SceneComponent.K2_SetRelativeLocation` _defaultsceneroot (`KismetMathLibrary.MakeVector` (+ _relativelocation_x (* (`self.Speed`) DeltaSeconds)) _relativelocation_y _relativelocation_z) false false)
    (else
      (`/Game/BluePrints/BP_SetActiveComponent.ActivateEvent` (`self.BP_SetActiveComponent`) false))))

(fn `UserConstructionScript`)