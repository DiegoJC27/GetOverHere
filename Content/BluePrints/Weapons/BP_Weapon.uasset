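; BP_Weapon is a weapon Blueprint that fires BP_Bullet actors repeatedly while the IA_Shoot input is ongoing.
; Each Ongoing trigger either calls Fire and resets TimeSinceLastShot once FireRate is reached, or adds the action's ElapsedSeconds to that timer.
; Fire spawns the bullet with the root's world rotation, at its world location plus an unrotated FireSocket offset.
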(event `EnhancedInput|/Game/BluePrints/IA_Shoot`
  (params (ActionValue :type Boolean) (ElapsedSeconds :type "Float (double-precision)") (TriggeredSeconds :type "Float (double-precision)") (InputAction :type "InputAction Object Reference" :default "/Game/BluePrints/IA_Shoot.IA_Shoot"))
  (:`Ongoing`
    (if (>= (`self.TimeSinceLastShot`) (`self.FireRate`))
      (set `self.TimeSinceLastShot` 0.0)
      (`self.Fire`)
      (else
        (set `self.TimeSinceLastShot` (+ ElapsedSeconds (`self.TimeSinceLastShot`)))))))

(event `Fire`
  (`|SpawnActorFromClass` "/Game/BluePrints/Weapons/BP_Bullet.BP_Bullet_C" (`KismetMathLibrary.MakeTransform` (+ (`self.FireSocket`) (`SceneComponent.K2_GetComponentLocation` (`self.DefaultSceneRoot`))) (`SceneComponent.K2_GetComponentRotation` (`self.DefaultSceneRoot`))) "Undefined" "MultiplyWithRoot" null null))

(fn `UserConstructionScript`)