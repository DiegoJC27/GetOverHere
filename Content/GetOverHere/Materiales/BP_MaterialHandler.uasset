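; Material handler that gives a set of meshes a runtime material with animated Fresnel and dither effects.
; ApplyRuntimeMaterial creates one dynamic instance from BaseMaterial, assigns it to every material slot on the given meshes, and resets both effect masks.
; Fresnel tweens its mask on or off, while Dither tweens its mask down to zero, both starting from the current value.
; The shared instance makes each effect change all those meshes together.
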(event `CreateRuntimeMaterial`
  (bind _returnvalue (`KismetMaterialLibrary.CreateDynamicMaterialInstance` (`self.BaseMaterial`)))
  (set `self.RuntimeMaterial` _returnvalue))

(event `ApplyRuntimeMaterial`
  (params (meshes :type "Array of MeshComponent Object Reference"))
  (bind _runtimematerial (`self.RuntimeMaterial`))
  (`self.CreateRuntimeMaterial`)
  (for _array_element meshes
    (for _index (range (+ (`PrimitiveComponent.GetNumMaterials` _array_element) 1))
      (`PrimitiveComponent.SetMaterial` _array_element _index _runtimematerial)
      (`MaterialInstanceDynamic.SetScalarParameterValue` _runtimematerial (`self.FresnelMask`) 0.0)
      (`MaterialInstanceDynamic.SetScalarParameterValue` _runtimematerial (`self.DitherMask`) 1.0))))

(event `Fresnel`
  (params (Active :type Boolean))
  (bind _runtimematerial (`self.RuntimeMaterial`))
  (bind _returnvalue (`MaterialInstanceDynamic.K2_GetScalarParameterValue` _runtimematerial (`self.FresnelMask`)))
  (bind (_asynctaskproxy _value) (`FCTweenBPActionFloat.TweenFloat` _returnvalue (`KismetMathLibrary.Conv_BoolToDouble` Active) 0.3)
    (:`ApplyEasing`
      (`MaterialInstanceDynamic.SetScalarParameterValue` _runtimematerial (`self.FresnelMask`) _value))))

(event `Dither`
  (bind _runtimematerial (`self.RuntimeMaterial`))
  (bind _returnvalue (`MaterialInstanceDynamic.K2_GetScalarParameterValue` _runtimematerial (`self.DitherMask`)))
  (bind (_asynctaskproxy _value) (`FCTweenBPActionFloat.TweenFloat` _returnvalue 0.0)
    (:`ApplyEasing`
      (`MaterialInstanceDynamic.SetScalarParameterValue` _runtimematerial (`self.DitherMask`) _value))))