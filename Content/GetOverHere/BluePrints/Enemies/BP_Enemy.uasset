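; Zombie enemy character that chases the player, attacks at close range, and can be deactivated and respawned for reuse.
; A recursive AI MoveTo loop follows the player pawn and triggers an attack montage within range, guarded by attacking and dying flags.
; Death sets the AnimBP flag, plays sound, stops movement and dithers the material, then deactivates after a delay through BPSetActiveComponent.
; Respawn reactivates and teleports the capsule.
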(event `self.ReceiveBeginPlay`
  (bind _bp_setactivecomponent (`self.BP_SetActiveComponent`))
  (`self.move`)
  (set `CharacterMovementComponent.MaxWalkSpeed` (`self.Speed`) (`self.CharacterMovement`))
  (add `/Game/GetOverHere/BluePrints/BP_SetActiveComponent.OnActiveEvent` _bp_setactivecomponent (delegate `Reset`))
  (`/Game/GetOverHere/BluePrints/BP_SetActiveComponent.SetActiveEvent` _bp_setactivecomponent true)
  (bind _asabp_enemy (cast `/Game/GetOverHere/BluePrints/Animaciones/Enemy/ABP_Enemy` (`SkeletalMeshComponent.GetAnimInstance` (`self.Mesh`))))
  (set `/Game/GetOverHere/BluePrints/Animaciones/Enemy/ABP_Enemy.Velocity` (`self.Speed`) _asabp_enemy)
  (`/Game/GetOverHere/Materiales/BP_MaterialHandler.ApplyRuntimeMaterial` (`self.BP_MaterialHandler`) (`|MakeArray` (`self.Mesh`) :!type "MeshComponent Object Reference")))

(event `Reset`
  (set `self.isActive` true))

(event `move`
  (if (not (`self.IsDying`))
    (`|AIMoveTo` self (0.0 0.0 0.0) (`GameplayStatics.GetPlayerPawn` 0)
      (:`OnSuccess`
        (`self.TryToAtack`)
        (`self.move`)))))

(event `TryToAtack`
  (if (`self.Atacking`)
    _
    (elif (not (> (`self.GetHorizontalDistanceTo` (`self.Player`)) 250.0))
      (`self.Atack`))))

(event `Atack`
  (if (not (`self.IsDying`))
    (set `self.Atacking` true)
    (`|PlayMontage` (`self.Mesh`) "/Game/GetOverHere/BluePrints/Animaciones/Enemy/AM_ZombieAtack.AM_ZombieAtack"
      (:`OnCompleted`
        (set `self.Atacking` false)))))

(event `Set player`
  (params (playerRef :type "/Game/GetOverHere/BluePrints/Player/BP_MyCharacter Object Reference"))
  (set `self.Player` playerRef))

(event `GetDirectionToPlayer`
  (params (DeltaTime :type "Float (double-precision)"))
  (set `self.Direction` (* (* (`KismetMathLibrary.Normal` (- (`SceneComponent.K2_GetComponentLocation` (`Character.CapsuleComponent` (`self.Player`))) (`SceneComponent.K2_GetComponentLocation` (`self.CapsuleComponent`)))) DeltaTime) (`self.Speed`))))

(event `Respawn`
  (params (transform :type "Transform Structure"))
  (`/Game/GetOverHere/BluePrints/BP_SetActiveComponent.SetActiveEvent` (`self.BP_SetActiveComponent`) true)
  (`SceneComponent.K2_SetWorldTransform` (`self.CapsuleComponent`) transform false true))

(event `OnZombieDie`
  (`self.Die`)
  (`KismetSystemLibrary.Delay` 2.0)
  (bind _output_get (set `self.isActive` false))
  (`/Game/GetOverHere/BluePrints/BP_SetActiveComponent.SetActiveEvent` (`self.BP_SetActiveComponent`) _output_get))

(fn `Die`
  (bind _asabp_enemy (cast `/Game/GetOverHere/BluePrints/Animaciones/Enemy/ABP_Enemy` (`SkeletalMeshComponent.GetAnimInstance` (`self.Mesh`))))
  (set `/Game/GetOverHere/BluePrints/Animaciones/Enemy/ABP_Enemy.IsDead` true _asabp_enemy)
  (`GameplayStatics.PlaySoundAtLocation` (`self.DieSound`) (`SceneComponent.K2_GetComponentLocation` (`self.CapsuleComponent`)) (struct) 1.0 1.0 0.0 null null null null)
  (set `self.IsDying` true)
  (`NavMovementInterface.StopActiveMovement` (`self.CharacterMovement`))
  (`/Game/GetOverHere/Materiales/BP_MaterialHandler.Dither` (`self.BP_MaterialHandler`)))

(fn `LookAt`
  (bind (_returnvalue_location _returnvalue_rotation) (`KismetMathLibrary.BreakTransform` (`self.GetTransform`)))
  (bind (_returnvalue_roll _returnvalue_pitch _returnvalue_yaw) (`KismetMathLibrary.BreakRotator` (`KismetMathLibrary.RInterpTo` _returnvalue_rotation (`KismetMathLibrary.FindLookAtRotation` _returnvalue_location (`self.K2_GetActorLocation` (`self.Player`))) (`GameplayStatics.GetWorldDeltaSeconds`) 1.0)))
  (`SceneComponent.K2_SetWorldRotation` (`self.Mesh`) (`KismetMathLibrary.MakeRotator` _returnvalue_roll _returnvalue_pitch (- _returnvalue_yaw 180.0)) false false))

(fn `UserConstructionScript`)