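; BP_LevelChanger is a portal trigger that moves the player to the next level or ends the game with a win.
; Initialize rebinds the player widget's dispatcher to its ChangeLevel event and plays the portal sound.
; Player overlap with the box calls WinGame on the widget if LastLevel is set, otherwise ChangeLevel on the game mode.
; LevelToOpen loads when the widget's dispatcher fires, not directly on overlap.
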(event `Initialize`
  (bind _asbp_my_game_mode (cast `/Game/GetOverHere/BluePrints/BP_MyGameMode` (`GameplayStatics.GetGameMode`)))
  (bind _playerwidget (`/Game/GetOverHere/BluePrints/BP_MyGameMode.PlayerWidget` _asbp_my_game_mode))
  (clear `/Game/GetOverHere/Widgets/WBP_PlayerUI.Dispatcher` _playerwidget)
  (add `/Game/GetOverHere/Widgets/WBP_PlayerUI.Dispatcher` _playerwidget (delegate `ChangeLevel`))
  (`GameplayStatics.PlaySoundAtLocation` (`self.PortalSound`) (`SceneComponent.K2_GetComponentLocation` (`self.DefaultSceneRoot`)) (struct) 1.0 1.0 0.0 null null null null))

(event `ChangeLevel`
  (`GameplayStatics.OpenLevelBySoftObjectPtr` (`self.LevelToOpen`)))

(event `self.BoxCol.OnComponentBeginOverlap`
  (params (OverlappedComponent :type "PrimitiveComponent Object Reference") (OtherActor :type "Actor Object Reference") (OtherComp :type "PrimitiveComponent Object Reference") (OtherBodyIndex :type Integer) (bFromSweep :type Boolean) (SweepResult :type "HitResult Structure (by ref)"))
  (cast `/Game/GetOverHere/BluePrints/Player/BP_MyCharacter` OtherActor)
  (bind _asbp_my_game_mode (cast `/Game/GetOverHere/BluePrints/BP_MyGameMode` (`GameplayStatics.GetGameMode`)))
  (if (`self.LastLevel`)
    (`/Game/GetOverHere/Widgets/WBP_PlayerUI.Win Game` (`/Game/GetOverHere/BluePrints/BP_MyGameMode.PlayerWidget` _asbp_my_game_mode))
    (else
      (`/Game/GetOverHere/BluePrints/BP_MyGameMode.ChangeLevel` _asbp_my_game_mode))))

(fn `UserConstructionScript`)