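; BP_EnemySpawner is an actor that spawns a set number of enemies, then spawns a level changer once none remain active.
; A Delay on Tick paces spawns at random choices among four transform offsets, handing each enemy the player reference and adding it to a pool.
; After the quota is met, it scans the pool's IsActive flags and spawns a single BP_LevelChanger configured with the level data.
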(event `self.ReceiveBeginPlay`
  (bind _asbp_my_character (cast `/Game/GetOverHere/BluePrints/Player/BP_MyCharacter` (`GameplayStatics.GetPlayerCharacter` 0)))
  (set `self.Player` _asbp_my_character))

(event `self.ReceiveTick`
  (params (DeltaSeconds :type "Float (single-precision)"))
  (bind (_output_location _output_rotation _output_scale) (`KismetMathLibrary.BreakTransform` (`|GetArrayItem` (`self.SpawnTransforms`))))
  (`KismetSystemLibrary.Delay` (`self.spawnCoolDown`))
  (if (> (`self.Enemies to Spawn`) (`self.Enemies spawned`))
    (`self.SpawnEnemy`)
    (elif (`self.NotSpawned`)
      (set `self.notEnded` false)
      (for _array_element (`self.EnemyPool`)
        (if (`/Game/GetOverHere/BluePrints/Enemies/BP_Enemy.isActive` _array_element)
          (set `self.notEnded` true)))
      (if (not (`self.notEnded`))
        (bind _returnvalue (`|SpawnActorFromClass` "/Game/GetOverHere/BluePrints/Enemies/BP_LevelChanger.BP_LevelChanger_C" (`KismetMathLibrary.MakeTransform` (+ (`SceneComponent.K2_GetComponentLocation` (`self.DefaultSceneRoot`)) _output_location) _output_rotation _output_scale) "AlwaysSpawn" "MultiplyWithRoot" null null))
        (set `/Game/GetOverHere/BluePrints/Enemies/BP_LevelChanger.LevelToOpen` (`self.curLevel`) _returnvalue)
        (`/Game/GetOverHere/BluePrints/Enemies/BP_LevelChanger.Initialize` _returnvalue)
        (set `/Game/GetOverHere/BluePrints/Enemies/BP_LevelChanger.LastLevel` (`self.IsLastLevel`) _returnvalue)
        (set `self.NotSpawned` false)))))

(event `SpawnEnemy`
  (bind _output_location (`KismetMathLibrary.BreakTransform` (`|GetArrayItem` (`self.SpawnTransforms`) (`KismetMathLibrary.RandomInteger` 4))))
  (bind _returnvalue (`|SpawnActorFromClass` "/Game/GetOverHere/BluePrints/Enemies/BP_Enemy.BP_Enemy_C" (`KismetMathLibrary.MakeTransform` (+ (`SceneComponent.K2_GetComponentLocation` (`self.DefaultSceneRoot`)) _output_location)) "AlwaysSpawn" "MultiplyWithRoot" null null))
  (`KismetArrayLibrary.Array_Add` (`self.EnemyPool`) _returnvalue)
  (`/Game/GetOverHere/BluePrints/Enemies/BP_Enemy.Set player` _returnvalue (`self.Player`))
  (set `self.Enemies spawned` (+ (`self.Enemies spawned`) 1)))

(fn `UserConstructionScript`)