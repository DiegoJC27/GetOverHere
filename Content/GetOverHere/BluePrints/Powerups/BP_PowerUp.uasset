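; BP_PowerUp is a pickup actor that triggers a power-up when a BP_MyCharacter overlaps it, then destroys itself.
; GivePlayerPowerUp receives the character but is empty here, so this Blueprint grants no effect itself.
; On BeginPlay, BPMaterialHandler applies a runtime material to the mesh and turns on a fresnel effect.
; Tick spins the root around yaw at a steady, frame-rate-independent speed, zeroing pitch and roll.
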(event `self.ReceiveBeginPlay`
  (bind _bp_materialhandler (`self.BP_MaterialHandler`))
  (`/Game/GetOverHere/Materiales/BP_MaterialHandler.ApplyRuntimeMaterial` _bp_materialhandler (`|MakeArray` (`self.Mesh`) :!type "MeshComponent Object Reference"))
  (`/Game/GetOverHere/Materiales/BP_MaterialHandler.Fresnel` _bp_materialhandler true))

(event `self.ReceiveActorBeginOverlap`
  (params (OtherActor :type "Actor Object Reference"))
  (bind _asbp_my_character (cast `/Game/GetOverHere/BluePrints/Player/BP_MyCharacter` OtherActor))
  (`self.GivePlayerPowerUp` _asbp_my_character)
  (`self.K2_DestroyActor`))

(event `self.ReceiveTick`
  (params (DeltaSeconds :type "Float (single-precision)"))
  (bind _defaultsceneroot (`self.DefaultSceneRoot`))
  (bind (_returnvalue_roll _returnvalue_pitch _returnvalue_yaw) (`KismetMathLibrary.BreakRotator` (`SceneComponent.K2_GetComponentRotation` _defaultsceneroot)))
  (`SceneComponent.K2_SetWorldRotation` _defaultsceneroot (`KismetMathLibrary.MakeRotator` 0.0 0.0 (+ _returnvalue_yaw (* DeltaSeconds 60.0))) false false))

(fn `GivePlayerPowerUp`
  (params (Player :type "/Game/GetOverHere/BluePrints/Player/BP_MyCharacter Object Reference")))

(fn `UserConstructionScript`)