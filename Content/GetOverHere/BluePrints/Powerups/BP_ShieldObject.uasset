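; BP_ShieldObject is a temporary powerup shield actor that circles the player and kills any BP_Enemy it overlaps through OnZombieDie.
; RecibePlayer stores the player reference that the orbit centers on.
; Tick advances an angle by Speed and uses sine and cosine to place the actor at Distance around the player's capsule, at capsule height.
; BeginPlay starts a Lifespan delay, after which the actor destroys itself.
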(event `self.ReceiveBeginPlay`
  (`KismetSystemLibrary.Delay` (`self.Lifespan`))
  (`self.K2_DestroyActor`))

(event `self.ReceiveActorBeginOverlap`
  (params (OtherActor :type "Actor Object Reference"))
  (bind _asbp_enemy (cast `/Game/GetOverHere/BluePrints/Enemies/BP_Enemy` OtherActor))
  (`/Game/GetOverHere/BluePrints/Enemies/BP_Enemy.OnZombieDie` _asbp_enemy))

(event `self.ReceiveTick`
  (params (DeltaSeconds :type "Float (single-precision)"))
  (bind (_returnvalue_x _returnvalue_y _returnvalue_z) (`KismetMathLibrary.BreakVector` (`SceneComponent.K2_GetComponentLocation` (`Character.CapsuleComponent` (`self.MyPlayer`)))))
  (bind _output_get (set `self.curDegree` (+ (`self.curDegree`) (* DeltaSeconds (`self.Speed`)))))
  (`SceneComponent.K2_SetWorldLocation` (`self.DefaultSceneRoot`) (`KismetMathLibrary.MakeVector` (+ (* (`KismetMathLibrary.DegCos` _output_get) (`self.Distance`)) _returnvalue_x) (+ _returnvalue_y (* (`KismetMathLibrary.DegSin` _output_get) (`self.Distance`))) _returnvalue_z) false false))

(fn `RecibePlayer`
  (params (Player :type "/Game/GetOverHere/BluePrints/Player/BP_MyCharacter Object Reference"))
  (set `self.MyPlayer` Player))

(fn `UserConstructionScript`)