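; Player character that moves on Enhanced Input axes, turns to face the mouse cursor and shoots.
; Each tick a camera-channel trace toward the deprojected cursor stores PointLookingAt and yaws only the mesh toward it, with a -90 degree offset.
; On BeginPlay it spawns a BP_Weapon, gives it a reference to itself and attaches it to the mesh's WeaponSocket.
; The shoot input calls TryShoot on that weapon.
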(event `self.ReceiveBeginPlay`
  (`self.Set Gun`))

(event `self.ReceiveTick`
  (params (DeltaSeconds :type "Float (single-precision)"))
  (`self.FollowCursor`))

(event `EnhancedInput|/Game/GetOverHere/BluePrints/IA_HorizontalMove`
  (params (ActionValue :type "Float (double-precision)") (ElapsedSeconds :type "Float (double-precision)") (TriggeredSeconds :type "Float (double-precision)") (InputAction :type "InputAction Object Reference" :default "/Game/GetOverHere/BluePrints/IA_HorizontalMove.IA_HorizontalMove"))
  (bind (_velocity_x _velocity_y _velocity_z) (`KismetMathLibrary.BreakVector` (`self.Velocity`)))
  (:`Triggered`
    (bind _output_get (set `self.Velocity` (`KismetMathLibrary.MakeVector` _velocity_x ActionValue _velocity_z)))
    (`self.AddMovementInput` (`KismetMathLibrary.MakeVector` (.x (stale `EnhancedInput|/Game/GetOverHere/BluePrints/IA_VerticalMove` _output_get)) (.y _output_get)) :!label _label)))

(event `EnhancedInput|/Game/GetOverHere/BluePrints/IA_VerticalMove`
  (params (ActionValue :type "Float (double-precision)") (ElapsedSeconds :type "Float (double-precision)") (TriggeredSeconds :type "Float (double-precision)") (InputAction :type "InputAction Object Reference" :default "/Game/GetOverHere/BluePrints/IA_VerticalMove.IA_VerticalMove"))
  (bind (_velocity_x _velocity_y _velocity_z) (`KismetMathLibrary.BreakVector` (`self.Velocity`)))
  (:`Triggered`
    (bind _output_get (set `self.Velocity` (`KismetMathLibrary.MakeVector` ActionValue _velocity_y _velocity_z)))
    (goto _label)))

(event `EnhancedInput|/Game/GetOverHere/BluePrints/IA_Shoot`
  (params (ActionValue :type Boolean) (ElapsedSeconds :type "Float (double-precision)") (TriggeredSeconds :type "Float (double-precision)") (InputAction :type "InputAction Object Reference" :default "/Game/GetOverHere/BluePrints/IA_Shoot.IA_Shoot"))
  (:`Triggered`
    (bind _activeweapon (`self.ActiveWeapon`)
      (:`then`
        (`/Game/GetOverHere/BluePrints/Weapons/BP_Weapon.Try Shoot` _activeweapon))
      (:`else`))))

(event `FollowCursor`
  (bind _returnvalue (`GameplayStatics.GetPlayerController` 0))
  (bind (_worldlocation _worlddirection) (`PlayerController.DeprojectMousePositionToWorld` _returnvalue))
  (bind (_returnvalue_location _returnvalue_rotation) (`KismetMathLibrary.BreakTransform` (`self.GetTransform` self)))
  (bind _outhit (`KismetSystemLibrary.LineTraceSingle` :`Start` (`self.K2_GetActorLocation` (`PlayerController.PlayerCameraManager` _returnvalue)) :`End` (* (+ _worldlocation (* _worlddirection 10000000.0)) 5000.0) :`TraceChannel` "TraceTypeQuery2" :`TraceColor` (struct :`R` 1.0 :`G` 0.052208 :`A` 1.0) :`DrawTime` 0.0))
  (set `self.PointLookingAt` (`.Location` (`GameplayStatics.BreakHitResult` _outhit)))
  (bind (_returnvalue_roll _returnvalue_pitch _returnvalue_yaw) (`KismetMathLibrary.BreakRotator` (`KismetMathLibrary.RInterpTo` _returnvalue_rotation (`KismetMathLibrary.FindLookAtRotation` _returnvalue_location (`.Location` (`GameplayStatics.BreakHitResult` _outhit))) (`GameplayStatics.GetWorldDeltaSeconds`))))
  (`SceneComponent.K2_SetWorldRotation` (`self.Mesh`) (`KismetMathLibrary.MakeRotator` 0.0 0.0 (- _returnvalue_yaw 90.0)) false false))

(event `Set Gun`
  (bind _returnvalue (`|SpawnActorFromClass` "/Game/GetOverHere/BluePrints/Weapons/BP_Weapon.BP_Weapon_C" (`self.GetTransform` self) "AlwaysSpawn" "MultiplyWithRoot" null null))
  (`self.SetOwner` _returnvalue _returnvalue)
  (set `self.ActiveWeapon` _returnvalue)
  (set `/Game/GetOverHere/BluePrints/Weapons/BP_Weapon.MyCharacter` self _returnvalue)
  (`self.K2_AttachToComponent` _returnvalue (`self.Mesh`) "WeaponSocket" "SnapToTarget" "SnapToTarget" "KeepRelative" true))

(fn `UserConstructionScript`)