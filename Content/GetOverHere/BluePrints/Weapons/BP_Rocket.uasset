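; BP_Rocket is an explosive projectile that extends a parent class's SetDirection and Collide logic.
; SetDirection calls the parent, then rotates the Sphere toward the target direction using look-at rotation with a yaw offset.
; Collide spawns an explosion, kills enemies and costs player characters a life within a sphere overlap radius.
; It also plays a sound and shakes the player's camera before calling the parent Collide.
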(event `self.Set Direction`
  (params (Start :type "Vector Structure") (End :type "Vector Structure"))
  (bind _sphere (`self.Sphere`))
  (bind (_returnvalue_location _returnvalue_rotation) (`KismetMathLibrary.BreakTransform` (`SceneComponent.K2_GetComponentToWorld` _sphere)))
  (bind (_returnvalue_roll _returnvalue_pitch _returnvalue_yaw) (`KismetMathLibrary.BreakRotator` (`KismetMathLibrary.FindLookAtRotation` _returnvalue_location (`self.Direction`))))
  (`parent.Set Direction` (`KismetMathLibrary.MakeVector` Start_X Start_Y Start_Z) End)
  (`SceneComponent.K2_SetWorldRotation` _sphere (`KismetMathLibrary.RInterpTo` _returnvalue_rotation (`KismetMathLibrary.MakeRotator` _returnvalue_roll _returnvalue_pitch (- _returnvalue_yaw 65.0))) false false))

(fn `Collide`
  (bind _returnvalue (`SceneComponent.K2_GetComponentLocation` (`self.Sphere`)))
  (`GameplayStatics.SpawnEmitterAtLocation` "/Game/FXVarietyPack/Particles/P_ky_explosion.P_ky_explosion" _returnvalue)
  (bind _outactors (`KismetSystemLibrary.SphereOverlapActors` _returnvalue (`self.Explsion radius`) (`self.Object Types`)))
  (for _array_element _outactors
    (bind _asbp_enemy (cast `/Game/GetOverHere/BluePrints/Enemies/BP_Enemy` _array_element)
      (:`then`
        (`/Game/GetOverHere/BluePrints/Enemies/BP_Enemy.OnZombieDie` _asbp_enemy))
      (:`CastFailed`
        (bind _asbp_my_character (cast `/Game/GetOverHere/BluePrints/Player/BP_MyCharacter` _array_element))
        (`/Game/GetOverHere/BluePrints/Player/BP_MyCharacter.LoseALife` _asbp_my_character))))
  (`GameplayStatics.PlaySoundAtLocation` (`self.ExplosionSound`) (`SceneComponent.K2_GetComponentLocation` (`self.Sphere`)) (struct) 1.0 1.0 0.0 null null null null)
  (bind _asbp_my_character_2 (cast `/Game/GetOverHere/BluePrints/Player/BP_MyCharacter` (`GameplayStatics.GetPlayerPawn` 0)))
  (`/Game/GetOverHere/BluePrints/Player/BP_MyCharacter.ShakeCamera` _asbp_my_character_2 2.0)
  (`parent.Collide`))

(fn `UserConstructionScript`
  (`parent.UserConstructionScript`))