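; Base-style weapon actor that fires bullets from its muzzle toward the character's aim point at a fixed height.
; TryShoot enforces a fire rate with a Tick-accumulated timer, then Fire spawns a bullet, plays sound, shakes the camera and updates ammo.
; Ammo updates the HUD through the game mode, and at zero the character switches to BP_RifleDeAsalto.
; Bullet pooling logic exists but is disconnected, so every shot spawns a new actor.
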(event `self.ReceiveBeginPlay`)

(event `Try Shoot`
  (if (>= (`self.TimeSinceLastShot`) (`self.FireRate`))
    (set `self.TimeSinceLastShot` 0.0)
    (`self.Fire`)))

(event `self.ReceiveTick`
  (params (DeltaSeconds :type "Float (single-precision)"))
  (set `self.TimeSinceLastShot` (+ DeltaSeconds (`self.TimeSinceLastShot`))))

(event `SpawnNewBullet`
  (bind (_returnvalue_location _returnvalue_rotation _returnvalue_scale) (`KismetMathLibrary.BreakTransform` (`SceneComponent.K2_GetComponentToWorld` (`self.Muzzle`))))
  (bind (_pointlookingat_x _pointlookingat_y) (`KismetMathLibrary.BreakVector` (`/Game/GetOverHere/BluePrints/Player/BP_MyCharacter.PointLookingAt` (`self.MyCharacter`))))
  (bind _returnvalue (`|SpawnActorFromClass` (`self.BulletType`) (`KismetMathLibrary.MakeTransform` _returnvalue_location _returnvalue_rotation _returnvalue_scale) "AlwaysSpawn" "MultiplyWithRoot" null null))
  (`/Game/GetOverHere/BluePrints/Weapons/BP_Bullet.Set Direction` _returnvalue _returnvalue_location (`KismetMathLibrary.MakeVector` _pointlookingat_x _pointlookingat_y (`self.BulletHeight`)))
  (`KismetArrayLibrary.Array_Add` (`self.BulletPool`) _returnvalue))

(event `Fire`
  (`self.SpawnNewBullet`)
  (`self.UpdateAmmo`)
  (`GameplayStatics.PlaySound2D` (`self.FireSound`) 1.0 1.0 0.0 null null)
  (`/Game/GetOverHere/BluePrints/Player/BP_MyCharacter.ShakeCamera` (`self.MyCharacter`) 0.2))

(fn `DestroyMySelf`
  (`self.K2_DestroyActor`))

(fn `SearchInPool`
  (returns (Found :type Boolean) (Bullet :type "/Game/GetOverHere/BluePrints/Weapons/BP_Bullet Object Reference"))
  (for _array_element (`self.BulletPool`)
    (`/Engine/EditorBlueprintResources/StandardMacros.IsValid` _array_element
      (:`Is Valid`
        (if (not (`/Game/GetOverHere/BluePrints/Weapons/BP_Bullet.IsActive` _array_element))
          (return true _array_element)))))
  (return false null))

(fn `UpdateAmmo`
  (bind _output_get (set `self.Ammo` (- (`self.Ammo`) 1)))
  (if (== _output_get 0)
    (`/Game/GetOverHere/BluePrints/Player/BP_MyCharacter.Set Gun` (`self.MyCharacter`) "/Game/GetOverHere/BluePrints/Weapons/BP_RifleDeAsalto.BP_RifleDeAsalto_C")
    (else
      (bind _asbp_my_game_mode (cast `/Game/GetOverHere/BluePrints/BP_MyGameMode` (`GameplayStatics.GetGameMode`)))
      (`/Game/GetOverHere/Widgets/WBP_PlayerUI.UpdateAmmoText` (`/Game/GetOverHere/BluePrints/BP_MyGameMode.PlayerWidget` _asbp_my_game_mode) (`self.Ammo`)))))

(fn `UserConstructionScript`)