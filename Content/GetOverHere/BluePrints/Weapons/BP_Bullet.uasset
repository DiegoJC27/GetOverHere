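; Projectile actor that kills any BP_Enemy it overlaps via OnZombieDie and destroys itself on contact with anything except BP_MyCharacter.
; SetDirection launches the physics Sphere with an acceleration-based force along the start-to-end direction.
; Activation through BPSetActiveComponent resets lifetime, velocity and position, and Tick destroys the active bullet when time expires.
; Despite this pooling-style reset, the deactivation nodes are disconnected, so bullets are destroyed rather than recycled.
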(event `self.ReceiveBeginPlay`
  (add `/Game/GetOverHere/BluePrints/BP_SetActiveComponent.OnActiveEvent` (`self.BP_SetActiveComponent`) (delegate `ResetBullet`))
  (set `self.TimeLeft` (`self.LifeSpan`)))

(event `ResetBullet`
  (bind _sphere (`self.Sphere`))
  (set `self.TimeLeft` (`self.LifeSpan`))
  (set `self.IsActive` true)
  (`PrimitiveComponent.SetPhysicsLinearVelocity` _sphere (0.0 0.0 0.0) false "None")
  (`SceneComponent.K2_SetRelativeLocation` _sphere (0.0 0.0 0.0) false true))

(event `self.ReceiveActorBeginOverlap`
  (params (OtherActor :type "Actor Object Reference"))
  (bind _asbp_enemy (cast `/Game/GetOverHere/BluePrints/Enemies/BP_Enemy` OtherActor)
    (:`then`
      (`/Game/GetOverHere/BluePrints/Enemies/BP_Enemy.OnZombieDie` _asbp_enemy))
    (:`CastFailed`
      (cast `/Game/GetOverHere/BluePrints/Player/BP_MyCharacter` OtherActor
        (:`CastFailed`
          _))))
  (`self.Collide`))

(event `Set Direction`
  (params (Start :type "Vector Structure") (End :type "Vector Structure"))
  (bind _output_get (set `self.Direction` (`KismetMathLibrary.Normal` (- End Start))))
  (`PrimitiveComponent.AddForce` (`self.Sphere`) (* _output_get (`self.Speed`)) "None" true))

(event `self.ReceiveTick`
  (params (DeltaSeconds :type "Float (single-precision)"))
  (if (`self.IsActive`)
    (bind _output_get (set `self.TimeLeft` (- (`self.TimeLeft`) DeltaSeconds)))
    (if (not (> _output_get 0.0))
      (`self.K2_DestroyActor`))))

(fn `Collide`
  (`self.K2_DestroyActor`))

(fn `UserConstructionScript`)