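; Game mode for GetOverHere that starts background music and tracks the current level number.
; On BeginPlay it shows the mouse cursor for the first player controller and plays the music as 2D sound.
; The ChangeLevel event increments the level counter, sets the player widget's "Nivel" label to the new number and calls EndLevel on that widget.
; The widget reference is not assigned in this Blueprint's graphs.
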(event `self.ReceiveBeginPlay`
  (set `PlayerController.bShowMouseCursor` true (`GameplayStatics.GetPlayerController` 0))
  (`GameplayStatics.PlaySound2D` (`self.BGMusic`) 1.0 1.0 0.0 null null))

(event `ChangeLevel`
  (bind _playerwidget (`self.PlayerWidget`))
  (bind _output_get (set `self.CurLevel` (+ (`self.CurLevel`) 1)))
  (`/Game/GetOverHere/Widgets/WBP_PlayerUI.SetCurLevelText` _playerwidget (`KismetTextLibrary.Conv_StringToText` (`KismetStringLibrary.Concat_StrStr` "Nivel " (`KismetStringLibrary.Conv_Int64ToString` _output_get))))
  (`/Game/GetOverHere/Widgets/WBP_PlayerUI.EndLevel` _playerwidget))

(fn `UserConstructionScript`)