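; Player character for a top-down shooter that moves on input, rotates to face the mouse cursor via a camera trace, and fires its active weapon.
; SetGun swaps the socket-attached weapon and updates the game mode's widget, and Tick feeds movement direction and magnitude to the AnimBP.
; LoseALife plays death animation, dither and camera shake, then respawns at the start with temporary invincibility or triggers game over.
; It can also spawn a shield power-up.
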(event `self.ReceiveBeginPlay`
  (`self.Set Gun` "/Game/GetOverHere/BluePrints/Weapons/BP_RifleDeAsalto.BP_RifleDeAsalto_C")
  (bind _asabp_player (cast `/Game/GetOverHere/BluePrints/Animaciones/Player/ABP_Player` (`SkeletalMeshComponent.GetAnimInstance` (`self.Mesh`))))
  (set `self.PlayerABP` _asabp_player)
  (set `self.StartingPos` (`SceneComponent.K2_GetComponentLocation` (`self.CapsuleComponent`)))
  (bind _asbp_my_game_mode (cast `/Game/GetOverHere/BluePrints/BP_MyGameMode` (`GameplayStatics.GetGameMode`)))
  (`/Game/GetOverHere/Widgets/WBP_PlayerUI.UpdateLifesText` (`/Game/GetOverHere/BluePrints/BP_MyGameMode.PlayerWidget` _asbp_my_game_mode) (`self.Lifes`))
  (`/Game/GetOverHere/Materiales/BP_MaterialHandler.ApplyRuntimeMaterial` (`self.BP_MaterialHandler`) (`|MakeArray` (`self.Mesh`) :!type "MeshComponent Object Reference")))

(event `self.ReceiveTick`
  (params (DeltaSeconds :type "Float (single-precision)"))
  (`self.FollowCursor`)
  (`self.UpdateAnimation`))

(event `EnhancedInput|/Game/GetOverHere/BluePrints/IA_HorizontalMove`
  (params (ActionValue :type "Float (double-precision)") (ElapsedSeconds :type "Float (double-precision)") (TriggeredSeconds :type "Float (double-precision)") (InputAction :type "InputAction Object Reference" :default "/Game/GetOverHere/BluePrints/IA_HorizontalMove.IA_HorizontalMove"))
  (bind (_velocity_x _velocity_y _velocity_z) (`KismetMathLibrary.BreakVector` (`self.Velocity`)))
  (:`Triggered`
    (if (not (`self.IsDying`))
      (bind _output_get (set `self.Velocity` (`KismetMathLibrary.MakeVector` _velocity_x ActionValue _velocity_z)))
      (`self.AddMovementInput` (`KismetMathLibrary.MakeVector` (.x (stale `EnhancedInput|/Game/GetOverHere/BluePrints/IA_VerticalMove` _output_get)) (.y _output_get)) :!label _label))))

(event `EnhancedInput|/Game/GetOverHere/BluePrints/IA_VerticalMove`
  (params (ActionValue :type "Float (double-precision)") (ElapsedSeconds :type "Float (double-precision)") (TriggeredSeconds :type "Float (double-precision)") (InputAction :type "InputAction Object Reference" :default "/Game/GetOverHere/BluePrints/IA_VerticalMove.IA_VerticalMove"))
  (bind (_velocity_x _velocity_y _velocity_z) (`KismetMathLibrary.BreakVector` (`self.Velocity`)))
  (:`Triggered`
    (if (not (`self.IsDying`))
      (bind _output_get (set `self.Velocity` (`KismetMathLibrary.MakeVector` ActionValue _velocity_y _velocity_z)))
      (goto _label))))

(event `EnhancedInput|/Game/GetOverHere/BluePrints/IA_Shoot`
  (params (ActionValue :type Boolean) (ElapsedSeconds :type "Float (double-precision)") (TriggeredSeconds :type "Float (double-precision)") (InputAction :type "InputAction Object Reference" :default "/Game/GetOverHere/BluePrints/IA_Shoot.IA_Shoot"))
  (:`Triggered`
    (if (not (`self.IsDying`))
      (bind _activeweapon (`self.ActiveWeapon`)
        (:`then`
          (`/Game/GetOverHere/BluePrints/Weapons/BP_Weapon.Try Shoot` _activeweapon))
        (:`else`)))))

(event `FollowCursor`
  (bind _returnvalue (`GameplayStatics.GetPlayerController` 0))
  (bind (_worldlocation _worlddirection) (`PlayerController.DeprojectMousePositionToWorld` _returnvalue))
  (bind (_returnvalue_location _returnvalue_rotation) (`KismetMathLibrary.BreakTransform` (`self.GetTransform` self)))
  (if (not (`self.IsDying`))
    (bind _outhit (`KismetSystemLibrary.LineTraceSingle` :`Start` (`self.K2_GetActorLocation` (`PlayerController.PlayerCameraManager` _returnvalue)) :`End` (* (+ _worldlocation (* _worlddirection 10000000.0)) 5000.0) :`TraceChannel` "TraceTypeQuery2" :`TraceColor` (struct :`R` 1.0 :`G` 0.052208 :`A` 1.0) :`DrawTime` 0.0))
    (set `self.PointLookingAt` (`.Location` (`GameplayStatics.BreakHitResult` _outhit)))
    (bind (_returnvalue_roll _returnvalue_pitch _returnvalue_yaw) (`KismetMathLibrary.BreakRotator` (`KismetMathLibrary.RInterpTo` _returnvalue_rotation (`KismetMathLibrary.FindLookAtRotation` _returnvalue_location (`.Location` (`GameplayStatics.BreakHitResult` _outhit))) (`GameplayStatics.GetWorldDeltaSeconds`))))
    (`self.K2_SetActorRotation` (`KismetMathLibrary.MakeRotator` 0.0 0.0 _returnvalue_yaw))))

(event `Respawn`
  (`SceneComponent.K2_SetWorldLocation` (`self.CapsuleComponent`) (`self.StartingPos`) false true)
  (bind _asabp_player (cast `/Game/GetOverHere/BluePrints/Animaciones/Player/ABP_Player` (`SkeletalMeshComponent.GetAnimInstance` (`self.Mesh`))))
  (set `/Game/GetOverHere/BluePrints/Animaciones/Player/ABP_Player.IsDead` false _asabp_player)
  (`MaterialInstanceDynamic.SetScalarParameterValue` (`/Game/GetOverHere/Materiales/BP_MaterialHandler.RuntimeMaterial` (`self.BP_MaterialHandler`)) "ditherMask" 1.0)
  (set `self.IsDying` false)
  (`self.Set Gun` "/Game/GetOverHere/BluePrints/Weapons/BP_RifleDeAsalto.BP_RifleDeAsalto_C")
  (`KismetSystemLibrary.Delay` (`self.Invincibility time`))
  (set `self.IsInvincible` false))

(event `Set Gun`
  (params (`NEW Weapon` :type "/Game/GetOverHere/BluePrints/Weapons/BP_Weapon Class Reference"))
  (bind _activeweapon (`self.ActiveWeapon`)
    (:`then`
      (`/Game/GetOverHere/BluePrints/Weapons/BP_Weapon.DestroyMySelf` _activeweapon))
    (:`else`
      _))
  (bind _returnvalue (`|SpawnActorFromClass` `NEW Weapon` (`self.GetTransform` self) "AlwaysSpawn" "MultiplyWithRoot" null null))
  (bind _asbp_my_game_mode (cast `/Game/GetOverHere/BluePrints/BP_MyGameMode` (`GameplayStatics.GetGameMode`)))
  (bind _playerwidget (`/Game/GetOverHere/BluePrints/BP_MyGameMode.PlayerWidget` _asbp_my_game_mode))
  (`/Game/GetOverHere/Widgets/WBP_PlayerUI.UpdateWeaponIcon` _playerwidget `NEW Weapon`)
  (`/Game/GetOverHere/Widgets/WBP_PlayerUI.UpdateAmmoText` _playerwidget (`/Game/GetOverHere/BluePrints/Weapons/BP_Weapon.Ammo` _returnvalue))
  (`self.SetOwner` _returnvalue _returnvalue)
  (set `self.ActiveWeapon` _returnvalue)
  (set `/Game/GetOverHere/BluePrints/Weapons/BP_Weapon.MyCharacter` self _returnvalue)
  (`self.K2_AttachToComponent` _returnvalue (`self.Mesh`) "WeaponSocket" "SnapToTarget" "SnapToTarget" "KeepRelative" true))

(event `LoseALife`
  (if (not (`self.IsInvincible`))
    (bind _output_get (set `self.Lifes` (- (`self.Lifes`) 1)))
    (bind _asabp_player (cast `/Game/GetOverHere/BluePrints/Animaciones/Player/ABP_Player` (`SkeletalMeshComponent.GetAnimInstance` (`self.Mesh`))))
    (set `/Game/GetOverHere/BluePrints/Animaciones/Player/ABP_Player.IsDead` true _asabp_player)
    (`/Game/GetOverHere/Materiales/BP_MaterialHandler.Dither` (`self.BP_MaterialHandler`))
    (`self.ShakeCamera` 1.0)
    (set `self.IsDying` true)
    (set `self.IsInvincible` true)
    (bind _asbp_my_game_mode (cast `/Game/GetOverHere/BluePrints/BP_MyGameMode` (`GameplayStatics.GetGameMode`)))
    (`/Game/GetOverHere/Widgets/WBP_PlayerUI.UpdateLifesText` (`/Game/GetOverHere/BluePrints/BP_MyGameMode.PlayerWidget` _asbp_my_game_mode) (`self.Lifes`))
    (`KismetSystemLibrary.Delay` 3.0)
    (if (> _output_get 0)
      (`self.Respawn`)
      (else
        (bind _asbp_my_game_mode_2 (cast `/Game/GetOverHere/BluePrints/BP_MyGameMode` (`GameplayStatics.GetGameMode`)))
        (`/Game/GetOverHere/Widgets/WBP_PlayerUI.Lose Game` (`/Game/GetOverHere/BluePrints/BP_MyGameMode.PlayerWidget` _asbp_my_game_mode_2))))))

(fn `ActivateShieldPowerUp`
  (bind _returnvalue (`|SpawnActorFromClass` "/Game/GetOverHere/BluePrints/Powerups/BP_ShieldObject.BP_ShieldObject_C" (`SceneComponent.K2_GetComponentToWorld` (`self.CapsuleComponent`)) "AlwaysSpawn" "MultiplyWithRoot" null null))
  (`/Game/GetOverHere/BluePrints/Powerups/BP_ShieldObject.RecibePlayer` _returnvalue self))

(fn `ShakeCamera`
  (params (NewParam :type "Float (double-precision)"))
  (set `self.Target Shake Scale` NewParam)
  (`PlayerCameraManager.StartCameraShake` :`self` (`PlayerController.PlayerCameraManager` (`GameplayStatics.GetPlayerController` 0)) :`ShakeClass` "/Game/GetOverHere/BluePrints/Animaciones/BP_CameraShake.BP_CameraShake_C" :`Scale` (`self.Target Shake Scale`)))

(fn `UpdateAnimation`
  (bind _playerabp (`self.PlayerABP`))
  (bind _returnvalue (`KismetMathLibrary.Normal` (`self.GetVelocity`)))
  (set `/Game/GetOverHere/BluePrints/Animaciones/Player/ABP_Player.Direction` (`KismetAnimationLibrary.CalculateDirection` _returnvalue (`self.K2_GetActorRotation`)) _playerabp)
  (set `/Game/GetOverHere/BluePrints/Animaciones/Player/ABP_Player.Magnitud` (`KismetMathLibrary.Abs` (`KismetMathLibrary.VSizeXY` _returnvalue)) _playerabp))

(fn `UserConstructionScript`)